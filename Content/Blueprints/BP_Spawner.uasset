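; Spawner actor that generates a continuous chain of BP_Platform actors at runtime.
; BeginPlay spawns a flagged initial platform, then the next one after a short delay.
; Each platform is placed past the previous one's tile-based width plus a random gap, with a randomized, clamped height.
; Non-initial platforms overlapping Trigger_Box each trigger one further spawn, guarded by their SpawnNext flag.
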(event OnComponentBeginOverlap(Trigger_Box)
  (params (OverlappedComponent :type Primitive%20Component%20Object%20Reference) (OtherActor :type Actor%20Object%20Reference) (OtherComp :type Primitive%20Component%20Object%20Reference) (OtherBodyIndex :type Integer) (bFromSweep :type Boolean) (SweepResult :type Hit%20Result%20Structure%20%28by%20ref%29))
  (bind _asbp_platform (Utilities|Casting|CastToBP_Platform OtherActor))
  (if (not (Variables|/Game/Blueprints/BP_Platform.BP_Platform_C|GetbInitialPlatform _asbp_platform))
    (if (not (Variables|/Game/Blueprints/BP_Platform.BP_Platform_C|GetbSpawnNext _asbp_platform))
      (Variables|/Game/Blueprints/BP_Platform.BP_Platform_C|SetbSpawnNext _asbp_platform true)
      (CallFunction|SpawnPlatforms))))

(event Custom|SpawnPlatforms
  (bind _returnvalue (Game|SpawnActorfromClass "/Game/Blueprints/BP_Platform.BP_Platform_C" (Math|Transform|MakeTransform (Math|Vector|MakeVector (+ (+ (.x (Transformation|GetActorLocation (Variables|Default|GetRef_Platform))) (* (Variables|/Game/Blueprints/BP_Platform.BP_Platform_C|GetTilesAmount (Variables|Default|GetRef_Platform)) 7e+01)) (Math|Random|RandomFloatinRange 1.5e+02 2.5e+02)) 1e+01 (Math|Float|Clamp(Float) (+ (.z (Transformation|GetActorLocation (Variables|Default|GetRef_Platform))) (Math|Random|RandomFloatinRange -1.5e+02 -2e+02)) -1.5e+02 -2e+02)) "0, 0, 0" "1,1,1") "AdjustIfPossibleButDontSpawnIfColliding" 0 false 0))
  (Variables|Default|SetRef_Platform _returnvalue))

(event EventBeginPlay
  (bind _returnvalue (Game|SpawnActorfromClass "/Game/Blueprints/BP_Platform.BP_Platform_C" (Math|Transform|MakeTransform (Math|Vector|MakeVector 2e+02 1e+01 (Math|Random|RandomFloatinRange -1.5e+02 -2e+02)) "0, 0, 0" "1,1,1") "AdjustIfPossibleButDontSpawnIfColliding" 0 true 0))
  (Variables|Default|SetRef_Platform _returnvalue)
  (Utilities|FlowControl|Delay 0.5)
  (CallFunction|SpawnPlatforms))

(event Collision|EventActorBeginOverlap
  (params (OtherActor :type Actor%20Object%20Reference)))

(fn ConstructionScript)