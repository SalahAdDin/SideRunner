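; BP_Platform is a 2D scrolling platform actor built from a row of box sprite tiles.
; On BeginPlay it adds Paper2D sprite components at even X spacing, using a fixed tile count for the initial platform and a random count for others.
; Each tile randomly picks one of two box sprites.
; Tick moves the whole actor along negative X at a constant, frame-rate-independent speed.
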(event EventBeginPlay
  (bind _output_get (Variables|Default|SetTilesAmount (select (Variables|Default|GetbInitialPlatform) 10 (Math|Random|RandomIntegerinRange 4 8))))
  (for _index (range 0 (- _output_get 1))
    (bind _returnvalue (AddComponent|AddPaperSpriteComponent false (Math|Transform|MakeTransform (Math|Vector|MakeVector (* _index 7e+01) 0.0 0.0) "0, 0, 0" "1,1,1")))
    (Rendering|Components|Sprite|SetSprite _returnvalue (select (Math|Random|RandomBool) "/Game/Textures/Sprites/box_Sprite.box_Sprite" "/Game/Textures/Sprites/boxAlt_Sprite.boxAlt_Sprite"))))

(event Collision|EventActorBeginOverlap
  (params (OtherActor :type Actor%20Object%20Reference)))

(event EventTick
  (params (DeltaSeconds :type Float%20%28single-precision%29))
  (Transformation|AddActorWorldOffset (Math|Vector|MakeVector (* DeltaSeconds -5e+02) 0.0 0.0)))

(fn ConstructionScript)