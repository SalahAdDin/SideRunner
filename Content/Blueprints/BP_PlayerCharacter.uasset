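; BP_PlayerCharacter is the player character, a sprite-based character with a double jump and a simple death event.
; Jump input performs a normal jump when grounded and arms one air jump, which launches the character upward by overriding vertical velocity.
; Tick calls Play on a Rotation timeline whose alpha drives the sprite's relative rotation.
; OnDeath sets the Death flag and destroys the actor.
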(event Custom|OnDeath
  (Variables|Default|SetbDeath true)
  (Actor|DestroyActor))

(event EventBeginPlay)

(event Collision|EventActorBeginOverlap
  (params (OtherActor :type Actor%20Object%20Reference)))

(event EventTick
  (params (DeltaSeconds :type Float%20%28single-precision%29))
  (bind _rotationalpha (Timeline|Rotation Play)
    (:Update
      (Transformation|SetRelativeRotation (Variables|Default|GetSprite) (Math|Rotator|MakeRotator 0.0 _rotationalpha 0.0) false false))))

(event Input|ActionEvents|InputActionJump
  (params (Key :type Key%20Structure :default "None"))
  (:Pressed
    (if (AI|Components|NavMovement|IsMovingonGround (Variables|Character|GetCharacterMovement))
      (Character|Jump)
      (Variables|Default|SetbDoubleJump true)
      (elif (Variables|Default|GetbDoubleJump)
        (Character|LaunchCharacter "0, 0,500.000000" false true)
        (Variables|Default|SetbDoubleJump false)))))

(fn ConstructionScript)