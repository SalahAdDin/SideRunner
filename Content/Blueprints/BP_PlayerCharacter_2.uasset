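; Player character for a side-runner game, with a rotating sprite, a jump with one mid-air double jump, and a death sequence.
; A Rotation timeline, played from Tick, drives sprite pitch, and a second air jump uses a vertical launch.
; OnDeath runs once, disabling collision, launching the character upward with a death spin, calling GameOver on BP_GM_SideRunner shortly after, and later freezing movement in flying mode.
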(event Custom|OnDeath
  (bind _charactermovement (Variables|Character|GetCharacterMovement))
  (if (not (Variables|Default|GetbDeath))
    (Utilities|FlowControl|Sequence
      (:then_0
        (Variables|Default|SetbDeath true)
        (Collision|SetActorEnableCollision false)
        (Character|LaunchCharacter "0, 0,1000.000000" true true)
        (bind _deathrotation (Timeline|OnDeathRotation Play)
          (:Update
            (Transformation|SetRelativeRotation (Variables|Default|GetSprite) (Math|Rotator|MakeRotator 0.0 _deathrotation 0.0) false false))))
      (:then_1
        (Utilities|FlowControl|Delay 0.2)
        (Default|GameOver (Variables|Default|GetRef_GameMode)))
      (:then_2
        (Utilities|FlowControl|Delay 4.0)
        (Pawn|Components|CharacterMovement|SetMovementMode _charactermovement "MOVE_Flying" 0)
        (Components|Movement|StopMovementImmediately _charactermovement)))))

(event EventBeginPlay
  (bind _asbp_gm_side_runner (Utilities|Casting|CastToBP_GM_SideRunner (Game|GetGameMode)))
  (Variables|Default|SetRef_GameMode _asbp_gm_side_runner))

(event Collision|EventActorBeginOverlap
  (params (OtherActor :type Actor%20Object%20Reference)))

(event EventTick
  (params (DeltaSeconds :type Float%20%28single-precision%29))
  (bind _rotationalpha (Timeline|Rotation Play)
    (:Update
      (Transformation|SetRelativeRotation (Variables|Default|GetSprite) (Math|Rotator|MakeRotator 0.0 _rotationalpha 0.0) false false))))

(event Input|ActionEvents|InputActionJump
  (params (Key :type Key%20Structure :default "None"))
  (:Pressed
    (if (AI|Components|NavMovement|IsMovingonGround (Variables|Character|GetCharacterMovement))
      (Character|Jump)
      (Variables|Default|SetbDoubleJump true)
      (elif (Variables|Default|GetbDoubleJump)
        (Character|LaunchCharacter "0, 0,500.000000" false true)
        (Variables|Default|SetbDoubleJump false)))))

(fn ConstructionScript)