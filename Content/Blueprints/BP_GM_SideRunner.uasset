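; BP_GM_SideRunner is the side runner's game mode, handling score, high score loading and HUD startup.
; BeginPlay caches the BP_GI_SideRunner game instance and calls its HUD widget function.
; UpdateScore increments the score and prints it as debug text.
; GetSaveGame loads the high score from the default BP_SaveCommon slot, or creates and saves a zeroed one if missing, then resets the current score.
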(event Custom|UpdateScore
  (bind _result (Math|Integer|IncrementInt (Variables|Default|GetScore))
    (:%20%20
      (Development|PrintString (Utilities|String|Append "Score: " (Utilities|String|ToString(Integer) _result))))))

(event Custom|GetSaveGame
  (bind _returnvalue (SaveGame|DoesSaveGameExist "Default"))
  (if _returnvalue
    (bind _returnvalue_2 (SaveGame|LoadGamefromSlot "Default"))
    (bind _asbp_save_common (Utilities|Casting|CastToBP_SaveCommon _returnvalue_2))
    (bind _output_get (Variables|Default|SetRef_SaveCommon _asbp_save_common))
    (Variables|Default|SetHighScore (Variables|/Game/Blueprints/BP_SaveCommon.BP_SaveCommon_C|GetHighScore _output_get))
    (else
      (bind _returnvalue_3 (SaveGame|CreateSaveGameObject "/Game/Blueprints/BP_SaveCommon.BP_SaveCommon_C"))
      (bind _output_get_2 (Variables|Default|SetRef_SaveCommon _returnvalue_3))
      (bind _output_get_3 (Variables|/Game/Blueprints/BP_SaveCommon.BP_SaveCommon_C|SetHighScore _output_get_2 0))
      (Variables|Default|SetHighScore _output_get_3)
      (SaveGame|SaveGametoSlot _returnvalue_3 "Default")))
  (Variables|Default|SetScore 0))

(event EventBeginPlay
  (Utilities|FlowControl|Sequence
    (:then_0
      (bind _asbp_gi_side_runner (Utilities|Casting|CastToBP_GI_SideRunner (Game|GetGameInstance)))
      (Variables|Default|SetRef_GameInstance _asbp_gi_side_runner))
    (:then_1
      (Default|CallHUDWBP (Variables|Default|GetRef_GameInstance)))))

(event EventTick
  (params (DeltaSeconds :type Float%20%28single-precision%29)))

(fn ConstructionScript)